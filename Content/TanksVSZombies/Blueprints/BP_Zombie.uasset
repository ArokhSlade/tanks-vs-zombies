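; Zombie Blueprint for TanksVSZombies that drives the enemy's 2D Paper2D flipbook animation through two events, ZombieWalk and ZombieAttack.
; ZombieWalk loops the walk flipbook and derives speed from distance moved per frame, scaling play rate between walk and run speeds.
; ZombieAttack plays the attack flipbook once from the start at normal rate.
; No movement or damage logic lives in this graph; BeginPlay, Tick and overlap events are empty.
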(event `self.ReceiveBeginPlay`)

(event `self.ZombieWalk`
  (params (DeltaSeconds :type "Float (single-precision)") (DistanceWalkedThisFrame :type "Vector Structure"))
  (bind _paperflipbook (`self.PaperFlipbook`))
  (bind _returnvalue (/ (`KismetMathLibrary.VSize` DistanceWalkedThisFrame) DeltaSeconds))
  (`PaperFlipbookComponent.SetFlipbook` _paperflipbook "/Game/TanksVSZombies/Sprites/Flipbooks/ZombieWalk.ZombieWalk")
  (`PaperFlipbookComponent.SetLooping` _paperflipbook true)
  (`PaperFlipbookComponent.Play` _paperflipbook)
  (`PaperFlipbookComponent.SetPlayRate` _paperflipbook (`KismetMathLibrary.MapRangeClamped` _returnvalue (`self.WalkSpeed`) (`self.RunSpeed`) 1.0 (`KismetMathLibrary.FClamp` (/ _returnvalue (`self.WalkSpeed`)) 1.0 (/ (`self.RunSpeed`) (`self.WalkSpeed`))))))

(event `self.ZombieAttack`
  (params (DeltaSeconds :type "Float (single-precision)"))
  (bind _paperflipbook (`self.PaperFlipbook`))
  (`PaperFlipbookComponent.SetFlipbook` _paperflipbook "/Game/TanksVSZombies/Sprites/Flipbooks/ZombieAttack.ZombieAttack")
  (`PaperFlipbookComponent.SetLooping` _paperflipbook false)
  (`PaperFlipbookComponent.PlayFromStart` _paperflipbook)
  (`PaperFlipbookComponent.SetPlayRate` _paperflipbook 1.0))

(fn `UserConstructionScript`)